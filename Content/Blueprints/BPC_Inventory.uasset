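; BPC_Inventory is an inventory component that stores item IDs and quantities in a Slots array.
; AddItem first looks for a matching slot below the MaxStack from DT_Items and adds the whole amount there, without clamping to that limit.
; If none is found, it fills the first slot with ItemID "None", and does nothing if no slot is free.
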(fn `AddItem`
  (params (ItemID :type Name) (Amount :type Integer))
  (locals (ItemAdded :type Boolean :default false))
  (bind _slots (`self.Slots`))
  (for (_array_element _array_index) (`self.Slots`)
    (bind _returnvalue (`|GetDataTableRow` "/Game/DataStructs/DT_Items.DT_Items" ItemID)
      (:`then`
        (bind (_itemid _quantity) (break `/Game/DataStructs/F_InventorySlot` _array_element))
        (if (and (== _itemid ItemID) (> (`.MaxStack_16_4F30798E4F99E8736022448EE2BE5B7D` (break `/Game/DataStructs/F_ItemData` _returnvalue)) _quantity))
          (`KismetArrayLibrary.Array_Set` (`self.Slots`) _array_index (make `/Game/DataStructs/F_InventorySlot` ItemID (+ _quantity Amount)))
          (set `local.ItemAdded` true)
          (break)))))
  (if (not (`local.ItemAdded`))
    (for (_array_element_2 _array_index_2) _slots
      (if (== (`.ItemID_2_31B2891840749DAD7D33C3A96B2B0E2C` (break `/Game/DataStructs/F_InventorySlot` _array_element_2)) "None")
        (`KismetArrayLibrary.Array_Set` _slots _array_index_2 (make `/Game/DataStructs/F_InventorySlot` ItemID Amount))
        (break)))))